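; BP_Playertest7 is a test player Blueprint that moves a physics body from axis input.
; MoveForward and MoveRight add force to the Player component along world X and Y respectively.
; Each force is the axis value times the body's mass times the Force variable, so acceleration stays independent of mass.
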(event `InputAxis|MoveRight`
  (params (AxisValue :type "Float (single-precision)"))
  (`PrimitiveComponent.AddForce` (`self.Player`) (`KismetMathLibrary.MakeVector` 0.0 (* AxisValue (* (`PrimitiveComponent.GetMass` (`self.Player`)) (`self.force`)))) "None" false))

(event `InputAxis|MoveForward`
  (params (AxisValue :type "Float (single-precision)"))
  (`PrimitiveComponent.AddForce` (`self.Player`) (`KismetMathLibrary.MakeVector` (* AxisValue (* (`PrimitiveComponent.GetMass` (`self.Player`)) (`self.force`)))) "None" false))

(fn `UserConstructionScript`)